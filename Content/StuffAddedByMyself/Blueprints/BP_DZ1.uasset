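; BP_DZ1 is an exercise Blueprint that, on BeginPlay, prints running sums of negative random integers.
; Each outer loop pass appends a random number, resizes Array to a fixed length and rescans it all.
; Negatives are written to Array2 without a varying index, and its contents are re-added to the total before each print, all inside nested loops.
; A disconnected first task holds a while-loop counter that never runs.
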(event EventBeginPlay
  (bind _array (Variables|Default|GetArray))
  (bind _array2 (Variables|Default|GetArray2))
  (Variables|Default|SetSumOfArray 0)
  (for _index (range 0 100)
    (Utilities|Array|Add _array (Math|Random|RandomIntegerinRange -100 100))
    (Utilities|Array|Resize _array 100)
    (for _array_element _array
      (if (< _array_element 0)
        (Utilities|Array|SetArrayElem _array2 0 _array_element true)
        (for _array_element_2 _array2
          (Variables|Default|SetSumOfArray (+ _array_element_2 (Variables|Default|GetSumOfArray))))
        (Development|PrintString (Utilities|String|ToString(Integer) (Variables|Default|GetSumOfArray)) true true "(R=0.794004,G=0.000000,B=1.000000,A=1.000000)" 1.8e+02)))))

(fn ConstructionScript)